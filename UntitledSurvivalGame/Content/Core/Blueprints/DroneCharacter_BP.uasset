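; Player-possessable drone character that becomes remotely controllable when someone interacts with it carrying a repair item, registering it with the game state's ControlNet.
; Non-heal damage unregisters it and returns the player to their original pawn, as does the swap input.
; While piloted it offers a remote HUD, flashlight, inventory, parts/task tracking and line-trace interaction cancelled by distance.
; A SceneCapture snapshots its view at BeginPlay, on unpossess and on request.
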(event `self.ReceiveBeginPlay`
  (`|ExecutionSequence`
    (:`then_0`
      (bind _asplayer_controller (cast `PlayerController` (`self.GetController`)))
      (bind _returnvalue (pcsubsystem `EnhancedInputLocalPlayerSubsystem` _asplayer_controller))
      (`/Engine/EditorBlueprintResources/StandardMacros.IsValid` _returnvalue
        (:`Is Valid`
          (message `EnhancedInputSubsystemInterface.AddMappingContext` _returnvalue "/Game/Core/Blueprints/Inputs/PlayerWalking_InputMap.PlayerWalking_InputMap" 1 (struct)))))
    (:`then_1`
      (`self.UpdateFlashlightGraphics`)
      (set `self.Info` (make `InteractionInfo` (`self.GetController`) self)))
    (:`then_2`
      (bind _asplayer_controller_2 (cast `PlayerController` (`self.GetController`)))
      (bind _returnvalue_2 (`|CreateWidget` "/Game/Core/UI/MapWidget.MapWidget_C" _asplayer_controller_2))
      (`UserWidget.AddToViewport` _returnvalue_2 0)
      (bind _returnvalue_3 (`|CreateWidget` "/Game/Dev/Test/TaskListWidget.TaskListWidget_C" _asplayer_controller_2))
      (`UserWidget.AddToViewport` _returnvalue_3 0)
      (set `self.TaskListWidget` _returnvalue_3)
      (`/Game/Dev/Test/TaskListWidget.UpdateLookupTable` (`self.TaskListWidget`) (`self.LookupTable`)))
    (:`then_3`
      (bind _returnvalue_4 (`|CreateWidget` "/Game/Core/Blueprints/Inventory/MenuInventory_Widget_BP.MenuInventory_Widget_BP_C" (cast `PlayerController` (`self.GetController`) :!pure true)))
      (`/Game/Core/Blueprints/Inventory/MenuInventory_Widget_BP.BuildWidget` _returnvalue_4 (`self.Inventory`))
      (set `InventoryComponent.InventoryWidget` _returnvalue_4 (`self.Inventory`)))
    (:`then_4`
      (`SceneCaptureComponent2D.CaptureScene` (`self.SceneCaptureComponent2D`))
      (set `self.DisplayName` (`|FormatText` "Drone: {ID}" (`KismetSystemLibrary.GetDisplayName` self))))
    (:`then_5`
      (cast `PlayerController` (`self.GetController`))
      (bind _outactors (`GameplayStatics.GetAllActorsOfClass` "DroneCharacter_BP_C"))
      (for _array_element _outactors
        (if (!= _array_element self)
          (bind _asdrone_character_bp (cast `/Game/Core/Blueprints/DroneCharacter_BP` _array_element))
          (set `self.LinkedPawn` _asdrone_character_bp)
          (set `/Game/Core/Blueprints/DroneCharacter_BP.LinkedPawn` self _asdrone_character_bp))))))

(event `CallSpawnItem`
  (params (Spawner :type "/Game/Dev/Test/PartSpawner Object Reference") (Amount :type Integer) (ClassRef :type "ItemAsset_Generic Class Reference"))
  (`/Game/Dev/Test/PartSpawner.SpawnItem` Spawner Amount ClassRef))

(event `CallPickupPart`
  (params (Name :type Name) (Amount :type Integer))
  (`self.PickupPart` Name Amount)
  (`KismetSystemLibrary.PrintString` "Picking up part?"))

(event `self.ReceiveTick`
  (params (DeltaSeconds :type "Float (single-precision)"))
  (bind _hit_actor (`self.Hit Actor`))
  (bind _info (`self.Info`))
  (set `SpringArmComponent.TargetArmLength` (* (`KismetMathLibrary.VSize` (- (`SceneComponent.K2_GetComponentLocation` (`self.Scene`)) (`SceneComponent.K2_GetComponentLocation` (`self.MaxLightDistance`)))) 0.5) (`self.SpringArm`))
  (if (not (`self.GetValidDistance`))
    (message `InteractionInterface.CancelInteraction` _hit_actor _info)
    (message `InteractionInterface.EndInteraction` _hit_actor _info)
    (set `self.Hit Actor` null)))

(event `EnhancedInput|/Game/Core/Blueprints/Inputs/Input_Flashlight`
  (params (ActionValue :type Boolean) (ElapsedSeconds :type "Float (double-precision)") (TriggeredSeconds :type "Float (double-precision)") (InputAction :type "InputAction Object Reference" :default "/Game/Core/Blueprints/Inputs/Input_Flashlight.Input_Flashlight"))
  (:`Triggered`
    (if (`self.IsFlashlightActive`)
      (set `self.IsFlashlightActive` false)
      (`self.UpdateFlashlightGraphics` :!label _label)
      (else
        (bind _canactivate (`self.CanFlshlightActivate`))
        (if _canactivate
          (set `self.IsFlashlightActive` true)
          (goto _label))))))

(event `EnhancedInput|/Game/Core/Blueprints/Inputs/Input_Interact`
  (params (ActionValue :type Boolean) (ElapsedSeconds :type "Float (double-precision)") (TriggeredSeconds :type "Float (double-precision)") (InputAction :type "InputAction Object Reference" :default "/Game/Core/Blueprints/Inputs/Input_Interact.Input_Interact"))
  (:`Started`
    (`self.StartInteraction`)))

(event `OnStartInteract`
  (params (Forward :type "Vector Structure"))
  (`SceneComponent.K2_SetWorldRotation` (`self.FirstPersonCameraComponent`) (`KismetMathLibrary.Conv_VectorToRotator` Forward) false false)
  (bind (_hit _hitactor) (`self.InteractionHandler`))
  (if (and _hit (`KismetSystemLibrary.DoesImplementInterface` _hitactor "/Script/InteractionSystem.InteractionInterface"))
    (set `self.Hit Actor` _hitactor)
    (set `self.LastHitLocation` (`.ImpactPoint` (`GameplayStatics.BreakHitResult` (`self.LastHit`))))
    (`/Engine/EditorBlueprintResources/StandardMacros.IsValid` (`self.Hit Actor`)
      (:`Is Valid`
        (message `InteractionInterface.BeginInteraction` (`self.Hit Actor`) (`self.Info`))))))

(event `OnCanceledInteract`
  (`/Engine/EditorBlueprintResources/StandardMacros.IsValid` (`self.Hit Actor`)
    (:`Is Valid`
      (message `InteractionInterface.CancelInteraction` (`self.Hit Actor`) (`self.Info`)))))

(event `OnCompletedInteract`
  (`/Engine/EditorBlueprintResources/StandardMacros.IsValid` (`self.Hit Actor`)
    (:`Is Valid`
      (message `InteractionInterface.EndInteraction` (`self.Hit Actor`) (`self.Info`)))))

(event `UpdateTasks_Needed`
  (params (Parts_Names :type "Array of Name") (Parts_Values :type "Array of Integer"))
  (bind _tasklistwidget (`self.TaskListWidget`))
  (`/Engine/EditorBlueprintResources/StandardMacros.IsValid` _tasklistwidget
    (:`Is Valid`
      (`/Game/Dev/Test/TaskListWidget.UpdateNeededItems` _tasklistwidget Parts_Names Parts_Values))))

(event `UpdateTasks_Held`
  (params (Names :type "Array of Name (by ref)") (Values :type "Array of Integer (by ref)"))
  (bind _tasklistwidget (`self.TaskListWidget`))
  (`/Engine/EditorBlueprintResources/StandardMacros.IsValid` _tasklistwidget
    (:`Is Valid`
      (`/Game/Dev/Test/TaskListWidget.UpdateHeldItems` _tasklistwidget Names Values))))

(event `self.UpdateCameraPitch`
  (params (Pitch :type "Float (single-precision)"))
  (`SceneComponent.K2_SetWorldRotation` (`self.Scene1`) (`KismetMathLibrary.MakeRotator` (.roll (`SceneComponent.K2_GetComponentRotation` (`self.FirstPersonCameraComponent`))) Pitch (.yaw (`SceneComponent.K2_GetComponentRotation` (`self.FirstPersonCameraComponent`)))) false false))

(event `EnhancedInput|/Game/Core/Blueprints/Inputs/Input_Inventory`
  (params (ActionValue :type Boolean) (ElapsedSeconds :type "Float (double-precision)") (TriggeredSeconds :type "Float (double-precision)") (InputAction :type "InputAction Object Reference" :default "/Game/Core/Blueprints/Inputs/Input_Inventory.Input_Inventory"))
  (:`Started`
    (`InventoryComponent.OpenInventoryWidget` (`self.Inventory`))))

(event `DropItem`
  (params (ItemData :type "ItemData Object Reference"))
  (`|SpawnActorFromClass` "/Game/Core/Blueprints/Inventory/BPSpawnedItem_Generic.BPSpawnedItem_Generic_C" (`KismetMathLibrary.Conv_VectorToTransform` (+ (`SceneComponent.K2_GetComponentLocation` (`self.FirstPersonCameraComponent`)) (* (`self.GetActorForwardVector`) 20.0))) "AdjustIfPossibleButAlwaysSpawn" "MultiplyWithRoot" null ItemData null))

(event `self.ReceiveAnyDamage`
  (params (Damage :type "Float (single-precision)") (DamageType :type "DamageType Object Reference") (InstigatedBy :type "Controller Object Reference") (DamageCauser :type "Actor Object Reference"))
  (if (> Damage 0.0)
    (if (not (`KismetMathLibrary.ClassIsChildOf` (`GameplayStatics.GetObjectClass` DamageType) "/Game/Core/Blueprints/Damage/DamageType_Heal.DamageType_Heal_C"))
      (bind _assurvival_player_controller_bp (cast `/Game/Core/Blueprints/SurvivalPlayerController_BP` (`self.GetController`)))
      (bind _assingleplayer_game_state (cast `/Game/Core/Blueprints/Game/SingleplayerGameState` (`GameplayStatics.GetGameState`)))
      (bind _ownedcontrolnet (`/Game/Core/Blueprints/Game/SingleplayerGameState.GetControlNet` _assingleplayer_game_state (`self.GetController`)))
      (`/Game/Core/Blueprints/Game/ControlNet.UnregisterControllableEntity` _ownedcontrolnet self)
      (`/Game/Core/Blueprints/SurvivalPlayerController_BP.ReturnToOriginalPawn` _assurvival_player_controller_bp)
      (set `self.IsRegistered` false))))

(event `EnhancedInput|/Game/Core/Blueprints/Inputs/Input_Crouch`
  (params (ActionValue :type Boolean) (ElapsedSeconds :type "Float (double-precision)") (TriggeredSeconds :type "Float (double-precision)") (InputAction :type "InputAction Object Reference" :default "/Game/Core/Blueprints/Inputs/Input_Crouch.Input_Crouch"))
  (:`Started`
    (`self.Crouch`))
  (:`Completed`
    (`self.UnCrouch`)))

(event `EnhancedInput|/Game/Core/Blueprints/Inputs/Input_Swap`
  (params (ActionValue :type Boolean) (ElapsedSeconds :type "Float (double-precision)") (TriggeredSeconds :type "Float (double-precision)") (InputAction :type "InputAction Object Reference" :default "/Game/Core/Blueprints/Inputs/Input_Swap.Input_Swap"))
  (:`Started`
    (bind _assurvival_player_controller_bp (cast `/Game/Core/Blueprints/SurvivalPlayerController_BP` (`self.GetController`)))
    (`/Game/Core/Blueprints/SurvivalPlayerController_BP.ReturnToOriginalPawn` _assurvival_player_controller_bp)))

(event `self.ReceivePossessed`
  (params (NewController :type "Controller Object Reference"))
  (`parent.ReceivePossessed` NewController)
  (bind _returnvalue (`|CreateWidget` "/Game/Core/UI/RemoteHUD.RemoteHUD_C"))
  (bind _output_get (set `self.W_RemoteHUD` _returnvalue))
  (`UserWidget.AddToViewport` _output_get 0))

(event `self.ReceiveUnpossessed`
  (params (OldController :type "Controller Object Reference"))
  (`Widget.RemoveFromParent` (`self.W_RemoteHUD`))
  (`SceneCaptureComponent2D.CaptureScene` (`self.SceneCaptureComponent2D`))
  (`parent.ReceiveUnpossessed` OldController))

(event `/Game/Core/Blueprints/Interfaces/RemoteControlInterface.CaptureView`
  (`SceneCaptureComponent2D.CaptureScene` (`self.SceneCaptureComponent2D`)))

(event `InteractionInterface.BeginInteraction`
  (params (Info :type "InteractionInfo Structure"))
  (bind ((`ControllerRef` _controllerref) (`PawnRef` _pawnref)) (break `InteractionInfo` Info))
  (bind _repairitem (`self.RepairItem`))
  (bind _returnvalue (`self.GetComponentByClass` _pawnref "/Script/UntitledSurvivalGame.InventoryComponent"))
  (if (`self.IsRegistered`)
    _
    (elif (`InventoryComponent.HasAmountOfItem` _returnvalue _repairitem 1)
      (bind _returnvalue_2 (`InventoryComponent.RemoveAmountOfTypeFromInventory` _returnvalue _repairitem 1))
      (if _returnvalue_2
        (bind _assingleplayer_game_state (cast `/Game/Core/Blueprints/Game/SingleplayerGameState` (`GameplayStatics.GetGameState`)))
        (bind _ownedcontrolnet (`/Game/Core/Blueprints/Game/SingleplayerGameState.GetControlNet` _assingleplayer_game_state _controllerref))
        (`/Game/Core/Blueprints/Game/ControlNet.RegisterControllableEntity` _ownedcontrolnet self)
        (set `self.IsRegistered` true))
      (else
        (`KismetSystemLibrary.PrintString` "Need override chip!")))))

(fn `CanFlshlightActivate`
  (returns (CanActivate :type Boolean))
  (return true))

(fn `CanInteract`
  (params (Info :type "InteractionInfo Structure"))
  (returns (ReturnValue :type Boolean))
  (return (not (`self.IsRegistered`))))

(fn `Get Parts`
  (returns (HeldParts :type "Map of Name to Integer"))
  (return (`self.Held Parts`)))

(fn `GetCameraComponent`
  (returns (ReturnValue :type "SceneComponent Object Reference"))
  (return (`self.FirstPersonCameraComponent`)))

(fn `GetLookatActor`
  (returns (LookatActor :type "Actor Object Reference"))
  (return (`.HitActor` (`GameplayStatics.BreakHitResult` (`self.LastCameraTraceResult`)))))

(fn `GetRemoteDisplayName`
  (returns (Name :type Text))
  (return (`self.DisplayName`)))

(fn `GetValidDistance`
  (returns (ReturnValue :type Boolean))
  (`/Engine/EditorBlueprintResources/StandardMacros.IsValid` (`self.Hit Actor`)
    (:`Is Valid`
      (return (<= (`KismetMathLibrary.Vector_Distance` (`SceneComponent.K2_GetComponentLocation` (`self.FirstPersonCameraComponent`)) (`self.LastHitLocation`)) (`self.InteractDistance`))))
    (:`Is Not Valid`
      (return true))))

(fn `InteractionHandler`
  (returns (Hit :type Boolean) (HitActor :type "Actor Object Reference"))
  (bind _firstpersoncameracomponent (`self.FirstPersonCameraComponent`))
  (bind _returnvalue (`SceneComponent.K2_GetComponentLocation` _firstpersoncameracomponent))
  (bind (_outhit _returnvalue_2) (`KismetSystemLibrary.LineTraceSingle` :`Start` _returnvalue :`End` (+ _returnvalue (* (`SceneComponent.GetForwardVector` _firstpersoncameracomponent) (`self.InteractDistance`))) :`TraceChannel` "TraceTypeQuery2" :`bTraceComplex` true :`DrawDebugType` "ForDuration"))
  (bind _output_get (set `self.LastHit` _outhit))
  (bind (_bblockinghit _binitialoverlap _time _distance _location _impactpoint _normal _impactnormal _physmat _hitactor _hitcomponent) (`GameplayStatics.BreakHitResult` _output_get))
  (bind _structout (setmembers `InteractionInfo` :`StructRef` (`self.Info`) :`HitComponent` _hitcomponent))
  (set `self.Info` _structout)
  (return _returnvalue_2 _hitactor))

(fn `IsCurrentlyControlled`
  (returns (ReturnValue :type Boolean))
  (return false))

(fn `OnRep_Held Parts_Values`
  (`BlueprintMapLibrary.Map_Clear` (`self.Held Parts`))
  (for (_array_element _array_index) (`self.Held Parts_Names`)
    (`BlueprintMapLibrary.Map_Add` (`self.Held Parts`) _array_element (`|GetArrayItem` (`self.Held Parts_Values`) _array_index)))
  (`KismetSystemLibrary.PrintString` "HeldPartsRep"))

(fn `OnRep_Hit Actor`
  (`/Engine/EditorBlueprintResources/StandardMacros.IsValid` (`self.Hit Actor`)
    (:`Is Valid`
      (`/Engine/EditorBlueprintResources/ActorMacros.Switch Has Authority`
        (:`Remote`
          (message `InteractionInterface.BeginInteraction` (`self.Hit Actor`) (`self.Info`)))))))

(fn `PickupPart`
  (params (Name :type Name) (Amount :type Integer))
  (returns (Success :type Boolean) (Remaining :type Integer))
  (if (> Amount 0)
    (`BlueprintMapLibrary.Map_Add` (`self.Held Parts`) Name (+ (`BlueprintMapLibrary.Map_Find` (`self.Held Parts`) Name) Amount))
    (`self.UpdateMap`)
    (`KismetSystemLibrary.PrintString` (`KismetStringLibrary.Concat_StrStr` "Pickup: " (`KismetStringLibrary.Conv_NameToString` Name)))
    (return true 0)
    (else
      (return false Amount))))

(fn `SetParts`
  (params (HeldParts :type "Map of Name to Integer"))
  (set `self.Held Parts` HeldParts)
  (`self.UpdateMap`)
  (return))

(fn `UpdateFlashlightGraphics`
  (bind _pointlight (`self.PointLight`))
  (bind _spotlight (`self.SpotLight`))
  (if (`self.IsFlashlightActive`)
    (`SceneComponent.SetVisibility` _spotlight true false)
    (`SceneComponent.SetVisibility` _pointlight true false)
    (else
      (`SceneComponent.SetVisibility` _spotlight false false)
      (`SceneComponent.SetVisibility` _pointlight false false))))

(fn `UpdateMap`
  (bind _held_parts (`self.Held Parts`))
  (bind _keys (`BlueprintMapLibrary.Map_Keys` _held_parts))
  (set `self.Held Parts_Names` _keys)
  (bind _values (`BlueprintMapLibrary.Map_Values` _held_parts))
  (set `self.Held Parts_Values` _values)
  (`self.UpdateTasks_Held` (`self.Held Parts_Names`) (`self.Held Parts_Values`)))

(fn `UserConstructionScript`)