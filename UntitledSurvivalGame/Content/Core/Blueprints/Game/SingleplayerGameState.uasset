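; Game state for singleplayer that sets up drone control at match start.
; BeginPlay constructs one ControlNet per player controller, then finds every DroneCharacter_BP and registers those flagged RegisterOnSpawn.
; Default drones always register as controllable entities with the first ControlNet.
; GetControlNet looks up the net owned by a given controller.
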(event `self.ReceiveBeginPlay`
  (for _index (range (`GameplayStatics.GetNumPlayerControllers`))
    (bind _returnvalue (`|GenericCreateObject` "/Game/Core/Blueprints/Game/ControlNet.ControlNet_C" (`GameplayStatics.GetPlayerController` _index)))
    (`KismetArrayLibrary.Array_Add` (`self.ControlNets`) _returnvalue))
  (bind _outactors (`GameplayStatics.GetAllActorsOfClass` "/Game/Core/Blueprints/DroneCharacter_BP.DroneCharacter_BP_C"))
  (for _array_element _outactors
    (if (`/Game/Core/Blueprints/DroneCharacter_BP.RegisterOnSpawn` _array_element)
      (`self.RegisterDefaultDrone` _array_element))))

(fn `GetControlNet`
  (params (Controller :type "Controller Object Reference"))
  (returns (OwnedControlNet :type "/Game/Core/Blueprints/Game/ControlNet Object Reference"))
  (for _array_element (`self.ControlNets`)
    (bind _returnvalue (`/Game/Core/Blueprints/Game/ControlNet.IsOwner` _array_element Controller))
    (if _returnvalue
      (return _array_element)))
  (return null))

(fn `RegisterDefaultDrone`
  (params (ActorRef :type "Actor Object Reference"))
  (`/Game/Core/Blueprints/Game/ControlNet.RegisterControllableEntity` (`|GetArrayItem` (`self.ControlNets`)) ActorRef))

(fn `UserConstructionScript`)