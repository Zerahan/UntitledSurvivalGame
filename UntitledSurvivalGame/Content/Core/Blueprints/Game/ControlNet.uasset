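; ControlNet is a registry of the pawns and other actors that can be controlled within one control network.
; Registering or unregistering sorts the actor by a Pawn cast into separate lists, messages it with a reference to the net, then fires OnUpdated.
; Query functions return either list or both combined, test membership, and check whether a controller is the owner or on the allow list.
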(event `RegisterControllableEntity`
  (params (ActorRef :type "Actor Object Reference"))
  (bind _aspawn (cast `Pawn` ActorRef)
    (:`then`
      (`KismetArrayLibrary.Array_AddUnique` (`self.ControllablePawns`) _aspawn)
      (message `/Game/Core/Blueprints/Interfaces/RemoteControlInterface.OnRegisteredWithControlNet` _aspawn self))
    (:`CastFailed`
      (`KismetArrayLibrary.Array_AddUnique` (`self.ControllableEntities`) ActorRef)
      (message `/Game/Core/Blueprints/Interfaces/RemoteControlInterface.OnRegisteredWithControlNet` ActorRef self)))
  (`self.OnUpdated` :!label _label))

(event `UnregisterControllableEntity`
  (params (ActorRef :type "Actor Object Reference"))
  (bind _aspawn (cast `Pawn` ActorRef)
    (:`then`
      (`KismetArrayLibrary.Array_RemoveItem` (`self.ControllablePawns`) _aspawn)
      (message `/Game/Core/Blueprints/Interfaces/RemoteControlInterface.OnUnregisteredWithControlNet` _aspawn self)
      (goto _label))
    (:`CastFailed`
      (`KismetArrayLibrary.Array_RemoveItem` (`self.ControllableEntities`))
      (message `/Game/Core/Blueprints/Interfaces/RemoteControlInterface.OnUnregisteredWithControlNet` ActorRef self)
      (goto _label))))

(fn `GetAllControlled`
  (returns (AllControlled :type "Array of Actor Object Reference"))
  (locals (LocalArray :type "Array of Actor Object Reference"))
  (`KismetArrayLibrary.Array_Append` (`local.LocalArray`) (`self.ControllableEntities`))
  (`KismetArrayLibrary.Array_Append` (`local.LocalArray`) (`self.ControllablePawns`))
  (return (`local.LocalArray`)))

(fn `GetControllableEntities`
  (returns (ControllableEntities :type "Array of Actor Object Reference"))
  (return (`self.ControllableEntities`)))

(fn `GetControllablePawns`
  (returns (ControllablePawns :type "Array of Pawn Object Reference"))
  (return (`self.ControllablePawns`)))

(fn `IsAllowListed`
  (params (Controller :type "Controller Object Reference"))
  (returns (ReturnValue :type Boolean))
  (return (`KismetArrayLibrary.Array_Contains` (`self.AllowedControllers`) Controller)))

(fn `IsEntityRegistered`
  (params (ActorRef :type "Actor Object Reference"))
  (returns (ReturnValue :type Boolean))
  (bind _aspawn (cast `Pawn` ActorRef)
    (:`then`
      (return (`KismetArrayLibrary.Array_Contains` (`self.ControllablePawns`) _aspawn)))
    (:`CastFailed`
      (return (`KismetArrayLibrary.Array_Contains` (`self.ControllableEntities`) ActorRef)))))

(fn `IsOwner`
  (params (Controller :type "Controller Object Reference"))
  (returns (ReturnValue :type Boolean))
  (return (== Controller (`self.OwningController`))))