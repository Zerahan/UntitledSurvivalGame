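; Game instance for the survival game that owns the settings and gameplay save objects, keyed by platform user name.
; On Init it loads or creates the user's settings save, which also records the last used slot.
; Loading a slot loads or creates its save, records that slot, then opens the saved map with the survival game mode and game-only input.
; Separate events write the current game or settings to disk.
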(event `self.ReceiveInit`
  (bind _returnvalue (`KismetStringLibrary.Concat_StrStr` (`self.GetUserName`) "_Settings"))
  (bind _returnvalue_2 (`GameplayStatics.DoesSaveGameExist` _returnvalue))
  (if _returnvalue_2
    (bind _returnvalue_3 (`GameplayStatics.LoadGameFromSlot` _returnvalue))
    (bind _assave_game_settings (cast `/Game/Core/Blueprints/Game/SaveGameSettings` _returnvalue_3))
    (set `self.SettingsSaveGame` _assave_game_settings)
    (else
      (bind _returnvalue_4 (`GameplayStatics.CreateSaveGameObject` "/Game/Core/Blueprints/Game/SaveGameSettings.SaveGameSettings_C"))
      (bind _output_get (set `self.SettingsSaveGame` _returnvalue_4))
      (`GameplayStatics.SaveGameToSlot` _output_get _returnvalue))))

(event `LoadGameFromSlot`
  (params (Slot :type String))
  (bind _returnvalue (`GameplayStatics.GetPlayerController` 0))
  (set `self.SaveSlot` (`KismetStringLibrary.Concat_StrStr` (`self.GetUserName`) "_" Slot))
  (bind _returnvalue_2 (`GameplayStatics.DoesSaveGameExist` (`self.SaveSlot`)))
  (if _returnvalue_2
    (bind _returnvalue_3 (`GameplayStatics.LoadGameFromSlot` (`self.SaveSlot`)))
    (set `self.SaveGameObject` _returnvalue_3)
    (else
      (bind _returnvalue_4 (`GameplayStatics.CreateSaveGameObject` "/Game/Core/Blueprints/Game/SurvivalSaveGame.SurvivalSaveGame_C"))
      (set `self.SaveGameObject` _returnvalue_4)
      (`self.SaveGameToSlot` (`self.SaveSlot`))))
  (set `/Game/Core/Blueprints/Game/SaveGameSettings.LastSaveSlot` Slot (`self.SettingsSaveGame`))
  (`self.SaveSettings`)
  (bind _assurvival_save_game (cast `/Game/Core/Blueprints/Game/SurvivalSaveGame` (`self.SaveGameObject`)))
  (`GameplayStatics.OpenLevel` (`/Game/Core/Blueprints/Game/SurvivalSaveGame.MapToLoad` _assurvival_save_game) true "Game=SurvivalGM_Base_BP")
  (`WidgetBlueprintLibrary.SetInputMode_GameOnly` _returnvalue)
  (set `PlayerController.bShowMouseCursor` false _returnvalue))

(event `SaveGame`
  (`self.SaveGameToSlot` (`self.SaveSlot`)))

(event `SaveGameToSlot`
  (params (Slot :type String))
  (`GameplayStatics.SaveGameToSlot` (`self.SaveGameObject`) Slot)
  (`KismetSystemLibrary.PrintString` "Hello"))

(event `SaveSettings`
  (bind _returnvalue (`GameplayStatics.SaveGameToSlot` (`self.SettingsSaveGame`) (`KismetStringLibrary.Concat_StrStr` (`self.GetUserName`) "_Settings")))
  (if _returnvalue
    (`KismetSystemLibrary.PrintString` "Saving settings....")
    (else
      (`KismetSystemLibrary.PrintString` "!!! Failed to save setttings !!!"))))

(fn `GetLastSaveSlot`
  (returns (UserName :type String) (LastSaveSlot :type String))
  (return (`self.GetUserName`) (`/Game/Core/Blueprints/Game/SaveGameSettings.LastSaveSlot` (`self.SettingsSaveGame`))))

(fn `GetSettingsSlotName`
  (returns (ReturnValue :type String))
  (return ""))

(fn `GetUserName`
  (returns (ReturnValue :type String))
  (return (`KismetSystemLibrary.GetPlatformUserName`)))