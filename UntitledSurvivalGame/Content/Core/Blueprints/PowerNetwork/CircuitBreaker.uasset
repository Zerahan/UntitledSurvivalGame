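; Interactable circuit breaker that controls a PowerNetwork, switching on only while its PowerStateDependencyActor supplies power.
; It lazily creates the network, registers as controller and zero-output generator, and reports a max power that can be randomized at BeginPlay.
; Toggling recalculates the network, whose power-state events can also set the breaker's state.
; Updates move the lever, recolor it green or red via a dynamic material, and display consumed, generated and max power.
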(event `self.ReceiveBeginPlay`
  (bind _returnvalue (`PrimitiveComponent.CreateDynamicMaterialInstance` (`self.Lever`) 0 (`PrimitiveComponent.GetMaterial` (`self.Lever`) 0) "None"))
  (bind _output_get (set `self.LeverColor_M` _returnvalue))
  (`PrimitiveComponent.SetMaterial` (`self.Lever`) 0 _output_get)
  (bind _network (`self.GetPoweredNetwork`))
  (bind _output_get_2 (set `self.NetworkRef` _network))
  (`/Game/Core/Blueprints/PowerNetwork/PowerNetwork.RegisterController` _output_get_2 self)
  (add `/Game/Core/Blueprints/PowerNetwork/PowerNetwork.OnUpdatedDispatcher` _output_get_2 (`|CreateDelegate` :!event `OnNetworkUpdated`))
  (add `/Game/Core/Blueprints/PowerNetwork/PowerNetwork.OnPowerStateUpdated` _output_get_2 (`|CreateDelegate` :!event `OnPowerStateUpdated`))
  (`|ExecutionSequence`
    (:`then_0`
      (if (and (!= (`self.MaxPowerHigh`) -1) (!= (`self.MaxPowerLow`) -1))
        (set `self.MaxPower` (`KismetMathLibrary.RandomIntegerInRange` (`self.MaxPowerLow`) (`self.MaxPowerHigh`)))))
    (:`then_1`
      (`self.UpdateGraphics`))))

(event `InteractionInterface.BeginInteraction`
  (params (Info :type "InteractionInfo Structure"))
  (bind _isactive (`self.GetParentPowerState`))
  (if _isactive
    (`self.SetIsPowered` (not (`self.IsPowered`)))
    (`KismetSystemLibrary.PrintString` (`KismetStringLibrary.Conv_BoolToString` _isactive))))

(event `OnNetworkUpdated`
  (`self.UpdateGraphics`))

(event `OnPowerStateUpdated`
  (params (IsPowered :type Boolean))
  (set `self.IsPowered` IsPowered)
  (`self.UpdateGraphics`))

(event `/Game/Core/Blueprints/PowerNetwork/TestPowerNetworkInterface.UpdatePowerState`
  (`self.SetIsPowered` (`self.IsPowered`)))

(fn `CanInteract`
  (params (Info :type "InteractionInfo Structure"))
  (returns (ReturnValue :type Boolean))
  (return true))

(fn `GetIsPowerActive`
  (params (InstigatingActor :type "Actor Object Reference"))
  (returns (IsActive :type Boolean))
  (return (`self.IsPowered`)))

(fn `GetIsReceivingPower`
  (returns (IsRecievingPower :type Boolean))
  (bind _powerstatedependencyactor (`self.PowerStateDependencyActor`))
  (`/Engine/EditorBlueprintResources/StandardMacros.IsValid` _powerstatedependencyactor
    (:`Is Valid`
      (bind _isactive (message `/Game/Core/Blueprints/PowerNetwork/TestPowerNetworkInterface.GetIsPowerActive` _powerstatedependencyactor self))
      (return _isactive))
    (:`Is Not Valid`
      (return false))))

(fn `GetMaxPower`
  (returns (MaxPower :type Integer))
  (return (`self.MaxPower`)))

(fn `GetParentPowerState`
  (returns (IsActive :type Boolean))
  (bind _powerstatedependencyactor (`self.PowerStateDependencyActor`))
  (`/Engine/EditorBlueprintResources/StandardMacros.IsValid` _powerstatedependencyactor
    (:`Is Valid`
      (bind _isactive (message `/Game/Core/Blueprints/PowerNetwork/TestPowerNetworkInterface.GetIsPowerActive` _powerstatedependencyactor self))
      (return _isactive))
    (:`Is Not Valid`
      (return false))))

(fn `GetPower`
  (returns (Power :type Integer))
  (return 0))

(fn `GetPoweredNetwork`
  (returns (Network :type "/Game/Core/Blueprints/PowerNetwork/PowerNetwork Object Reference"))
  (`/Engine/EditorBlueprintResources/StandardMacros.IsValid` (`self.NetworkRef`)
    (:`Is Valid`
      _)
    (:`Is Not Valid`
      (bind _returnvalue (`|GenericCreateObject` "/Game/Core/Blueprints/PowerNetwork/PowerNetwork.PowerNetwork_C"))
      (bind _output_get (set `self.NetworkRef` _returnvalue))
      (`/Game/Core/Blueprints/PowerNetwork/PowerNetwork.RegisterGenerator` _output_get self 0)
      (add `/Game/Core/Blueprints/PowerNetwork/PowerNetwork.OnUpdatedDispatcher` _output_get (`|CreateDelegate` :!event `OnNetworkUpdated`))))
  (return (`self.NetworkRef`)))

(fn `SetIsPowered`
  (params (IsPowered :type Boolean))
  (bind _isrecievingpower (`self.GetIsReceivingPower`))
  (set `self.IsPowered` (and _isrecievingpower IsPowered))
  (bind _network (`self.GetPoweredNetwork`))
  (`/Game/Core/Blueprints/PowerNetwork/PowerNetwork.Recalculate` _network)
  (`self.UpdateGraphics`))

(fn `UpdateGraphics`
  (bind _networkref (`self.NetworkRef`))
  (bind _returnvalue (and (`self.GetParentPowerState`) (`self.IsPowered`)))
  (`|ExecutionSequence`
    (:`then_0`
      (`/Engine/EditorBlueprintResources/StandardMacros.IsValid` (`self.LeverColor_M`)
        (:`Is Valid`
          (`MaterialInstanceDynamic.SetVectorParameterValue` (`self.LeverColor_M`) "Color" (`KismetMathLibrary.SelectColor` (struct :`G` 1.0 :`A` 1.0) (struct :`R` 1.0 :`A` 1.0) _returnvalue))
          (`SceneComponent.K2_SetRelativeLocation` (`self.Lever`) (`KismetMathLibrary.SelectVector` (8.0 0.0 -40.0) (8.0 0.0 40.0) _returnvalue) false false))))
    (:`then_1`
      (`TextRenderComponent.K2_SetText` (`self.TextRender`) (`|FormatText` "{Consumed} / {Generated} \n{Max}" (`/Game/Core/Blueprints/PowerNetwork/PowerNetwork.TotalConsumed` _networkref) (`/Game/Core/Blueprints/PowerNetwork/PowerNetwork.TotalGenerated` _networkref) (`self.MaxPower`))))))

(fn `UserConstructionScript`)