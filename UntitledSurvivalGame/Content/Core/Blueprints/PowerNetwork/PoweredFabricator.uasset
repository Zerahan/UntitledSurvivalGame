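; Powered fabricator actor in the power network folder that outputs items into the world as spawned item actors.
; Its SpawnItem event wraps the given item class and amount in a new quantity item data object.
; That data is passed to a generic spawned item actor, owned by the fabricator and always spawned at the SpawnPoint's location and rotation.
; The construction script only calls its parent.
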(event `SpawnItem`
  (params (Amount :type Integer) (ItemClass :type "ItemAsset_Generic Class Reference"))
  (bind _returnvalue (`|GenericCreateObject` "/Script/UntitledSurvivalGame.ItemData_Quantity"))
  (set `ItemData.ClassRef` ItemClass _returnvalue)
  (set `ItemData_Quantity.Amount` Amount _returnvalue)
  (`|SpawnActorFromClass` "/Game/Core/Blueprints/Inventory/BPSpawnedItem_Generic.BPSpawnedItem_Generic_C" (`KismetMathLibrary.MakeTransform` (.location (`SceneComponent.K2_GetComponentToWorld` (`self.SpawnPoint`))) (.rotation (`SceneComponent.K2_GetComponentToWorld` (`self.SpawnPoint`)))) "AlwaysSpawn" "MultiplyWithRoot" self _returnvalue null))

(fn `UserConstructionScript`
  (`parent.UserConstructionScript`))