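; Power network that tracks registered generators, consumers and controllers and decides whether the network is powered.
; Each registration change triggers Recalculate, which totals generation and consumption by querying members directly rather than reading the stored power arrays.
; Power requires every controller to be active with sufficient capacity for total consumption, and generation to cover consumption.
; Dispatchers then broadcast the update and resulting power state.
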(event `RegisterGenerator`
  (params (GeneratorRef :type "Actor Object Reference") (GeneratedAmount :type Integer))
  (bind _returnvalue (`KismetArrayLibrary.Array_AddUnique` (`self.Generators`) GeneratorRef))
  (if (!= _returnvalue -1)
    (`KismetArrayLibrary.Array_Set` (`self.GeneratedPower`) _returnvalue GeneratedAmount true)
    (`self.Recalculate`)))

(event `UnregisterGenerator`
  (params (Item :type "Actor Object Reference (by ref)"))
  (bind _returnvalue (`KismetArrayLibrary.Array_Find` (`self.Generators`) Item))
  (if (!= _returnvalue -1)
    (`KismetArrayLibrary.Array_Remove` (`self.GeneratedPower`) _returnvalue)
    (`KismetArrayLibrary.Array_RemoveItem` (`self.Generators`) Item)
    (`self.Recalculate`)))

(event `RegisterConsumer`
  (params (ConsumerRef :type "Actor Object Reference (by ref)") (ConsumedAmount :type Integer))
  (bind _returnvalue (`KismetArrayLibrary.Array_AddUnique` (`self.Consumers`) ConsumerRef))
  (if (!= _returnvalue -1)
    (`KismetArrayLibrary.Array_Set` (`self.ConsumedPower`) _returnvalue ConsumedAmount true)
    (`self.Recalculate`)))

(event `UnregisterConsumer`
  (params (Item :type "Actor Object Reference (by ref)"))
  (bind _returnvalue (`KismetArrayLibrary.Array_Find` (`self.Consumers`) Item))
  (if (!= _returnvalue -1)
    (`KismetArrayLibrary.Array_Remove` (`self.ConsumedPower`) _returnvalue)
    (`KismetArrayLibrary.Array_RemoveItem` (`self.Consumers`) Item)
    (`self.Recalculate`)))

(event `RegisterController`
  (params (ControllerRef :type "Actor Object Reference"))
  (`KismetArrayLibrary.Array_AddUnique` (`self.Controllers`) ControllerRef)
  (`self.Recalculate`))

(event `Unregister Controller`
  (params (Item :type "Actor Object Reference"))
  (if (!= (`KismetArrayLibrary.Array_Find` (`self.Controllers`) Item) -1)
    (`KismetArrayLibrary.Array_RemoveItem` (`self.Consumers`) Item)
    (`self.Recalculate`)))

(fn `Recalculate`
  (locals (CanIsPowered :type Boolean))
  (`|ExecutionSequence`
    (:`then_0`
      (set `self.TotalGenerated` 0)
      (for _array_element (`self.Generators`)
        (bind _power (message `/Game/Core/Blueprints/PowerNetwork/TestPowerNetworkInterface.GetPower` _array_element))
        (set `self.TotalGenerated` (+ _power (`self.TotalGenerated`)))))
    (:`then_1`
      (set `self.TotalConsumed` 0)
      (for _array_element_2 (`self.Consumers`)
        (bind _power_2 (message `/Game/Core/Blueprints/PowerNetwork/TestPowerNetworkInterface.GetPower` _array_element_2))
        (set `self.TotalConsumed` (+ _power_2 (`self.TotalConsumed`)))))
    (:`then_2`
      (set `local.CanIsPowered` true)
      (for _array_element_3 (`self.Controllers`)
        (bind _isactive (message `/Game/Core/Blueprints/PowerNetwork/TestPowerNetworkInterface.GetIsPowerActive` _array_element_3 null))
        (if _isactive
          (bind _maxpower (message `/Game/Core/Blueprints/PowerNetwork/TestPowerNetworkInterface.GetMaxPower` _array_element_3))
          (if (> (`self.TotalConsumed`) _maxpower)
            (set `local.CanIsPowered` false :!label _label))
          (else
            (goto _label)))))
    (:`then_3`
      (`self.OnUpdatedDispatcher`))
    (:`then_4`
      (`self.OnPowerStateUpdated` (and (`local.CanIsPowered`) (>= (`self.TotalGenerated`) (`self.TotalConsumed`)))))))