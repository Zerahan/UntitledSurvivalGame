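; Interactable power-consumer actor that opens a menu widget when it is receiving power and switched on.
; It registers with the power network of its PoweredActor and derives its received-power state from that actor.
; A child devSwitch toggles its active state and triggers network recalculation, while interacting elsewhere on a powered but inactive actor switches it on.
; A text render and the switch display the current state.
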(event `self.ReceiveBeginPlay`
  (`|ExecutionSequence`
    (:`then_0`
      (`/Engine/EditorBlueprintResources/StandardMacros.IsValid` (`self.PoweredActor`)
        (:`Is Valid`
          (bind _network (message `/Game/Core/Blueprints/PowerNetwork/TestPowerNetworkInterface.GetPoweredNetwork` (`self.PoweredActor`)))
          (bind _output_get (set `self.PowerNetworkRef` _network))
          (`/Game/Core/Blueprints/PowerNetwork/PowerNetwork.RegisterConsumer` _output_get self (`self.ConsumedPower`))
          (add `/Game/Core/Blueprints/PowerNetwork/PowerNetwork.OnPowerStateUpdated` _output_get (`|CreateDelegate` :!event `OnPowerNetworkStateUpdated`)))))
    (:`then_1`
      (`self.UpdateGraphics`)
      (bind _asdev_switch (cast `/Game/Dev/PowerSystems/devSwitch` (`ChildActorComponent.ChildActor` (`self.ChildActor`))))
      (add `/Game/Dev/PowerSystems/devSwitch.OnSwitchUpdated` _asdev_switch (`|CreateDelegate` :!event `OnSwitchUpdated`)))))

(event `InteractionInterface.BeginInteraction`
  (params (Info :type "InteractionInfo Structure"))
  (if (== (`KismetSystemLibrary.GetOuterObject` (`.HitComponent` (break `InteractionInfo` Info))) (`self.ChildActor`))
    (`self.OnSwitchUpdated` (not (`self.IsPowerActive`)))
    (elif (`self.IsRecievingPower`)
      (if (`self.IsPowerActive`)
        (bind _asplayer_controller (cast `PlayerController` (`.ControllerRef` (break `InteractionInfo` Info))))
        (if (`KismetSystemLibrary.IsValidClass` (`self.MenuWidgetToOpen`))
          (bind _returnvalue (`|CreateWidget` (`self.MenuWidgetToOpen`) _asplayer_controller self))
          (`UserWidget.AddToViewport` _returnvalue 0))
        (else
          (set `self.IsPowerActive` true)
          (`/Game/Core/Blueprints/PowerNetwork/PowerNetwork.Recalculate` (`self.PowerNetworkRef`)))))))

(event `OnPowerNetworkStateUpdated`
  (params (IsPowered :type Boolean))
  (bind _isactive (`self.GetIsPowerActive` null))
  (`self.SetIsPowerActive` _isactive))

(event `OnSwitchUpdated`
  (params (IsSwitchOn :type Boolean))
  (set `self.IsPowerActive` IsSwitchOn)
  (`/Game/Core/Blueprints/PowerNetwork/PowerNetwork.Recalculate` (`self.PowerNetworkRef`))
  (`self.UpdateGraphics`))

(fn `CanInteract`
  (params (Info :type "InteractionInfo Structure"))
  (returns (ReturnValue :type Boolean))
  (return true))

(fn `GetIsPowerActive`
  (params (InstigatingActor :type "Actor Object Reference"))
  (returns (IsActive :type Boolean))
  (return (`self.IsPowerActive`)))

(fn `GetIsReceivingPower`
  (returns (IsRecievingPower :type Boolean))
  (bind _isactive (message `/Game/Core/Blueprints/PowerNetwork/TestPowerNetworkInterface.GetIsPowerActive` (`self.PoweredActor`) self))
  (set `self.IsRecievingPower` _isactive)
  (return (`self.IsRecievingPower`)))

(fn `GetMaxPower`
  (returns (MaxPower :type Integer))
  (return 0))

(fn `GetPower`
  (returns (Power :type Integer))
  (return (`KismetMathLibrary.SelectInt` (`self.ConsumedPower`) 0 (`self.IsPowerActive`))))

(fn `GetPoweredNetwork`
  (returns (Network :type "/Game/Core/Blueprints/PowerNetwork/PowerNetwork Object Reference"))
  (return (`self.PowerNetworkRef`)))

(fn `SetIsPowerActive`
  (params (IsPowerActive :type Boolean))
  (bind _isrecievingpower (`self.GetIsReceivingPower`))
  (set `self.IsPowerActive` (and _isrecievingpower IsPowerActive)))

(fn `UpdateGraphics`
  (`TextRenderComponent.K2_SetText` (`self.TextRender`) (`|FormatText` "{a}{b}" (`KismetTextLibrary.Conv_StringToText` (select `bool` (`self.IsRecievingPower`) :`false` "o" :`true` "-")) (`KismetTextLibrary.Conv_StringToText` (select `bool` (`self.IsPowerActive`) :`false` "o" :`true` "-"))))
  (bind _asdev_switch (cast `/Game/Dev/PowerSystems/devSwitch` (`ChildActorComponent.ChildActor` (`self.ChildActor`))))
  (`/Game/Dev/PowerSystems/devSwitch.SetSwitchState` _asdev_switch (`self.IsPowerActive`)))

(fn `UserConstructionScript`)