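; Interactable power generator that supplies a fixed or randomized amount of power to a PowerNetwork and can be toggled on and off.
; It joins its parent generator's network at BeginPlay, or lazily constructs its own when none is set.
; Toggling recalculates the network and recolors a dynamic-material indicator light green or red.
; Text renders show its output and, on network update events, consumed versus generated totals while powered.
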(event `self.ReceiveBeginPlay`
  (bind _indicatorlight_sm (`self.IndicatorLight_SM`))
  (bind _parentgenerator (`self.ParentGenerator`))
  (`|ExecutionSequence`
    (:`then_0`
      (bind _returnvalue (`PrimitiveComponent.CreateDynamicMaterialInstance` _indicatorlight_sm 0 (`PrimitiveComponent.GetMaterial` _indicatorlight_sm 0) "None"))
      (bind _output_get (set `self.IndicatorLight_MAT` _returnvalue))
      (`PrimitiveComponent.SetMaterial` (`self.IndicatorLight_SM`) 0 _output_get)
      (`self.UpdateGraphics`))
    (:`then_1`
      (if (and (!= (`self.GeneratedPower_Min`) -1) (!= (`self.GeneratedPower_Max`) -1))
        (set `self.GeneratedPower` (`KismetMathLibrary.RandomIntegerInRange` (`self.GeneratedPower_Min`) (`self.GeneratedPower_Max`))))
      (`TextRenderComponent.K2_SetText` (`self.TextRender1`) (`|FormatText` "+{A}" (`KismetTextLibrary.Conv_IntToText` (`self.GeneratedPower`))))
      (`/Engine/EditorBlueprintResources/StandardMacros.IsValid` _parentgenerator
        (:`Is Valid`
          (bind _network (message `/Game/Core/Blueprints/PowerNetwork/TestPowerNetworkInterface.GetPoweredNetwork` _parentgenerator))
          (bind _output_get_2 (set `self.NetworkRef` _network))
          (`/Game/Core/Blueprints/PowerNetwork/PowerNetwork.RegisterGenerator` _output_get_2 self (`self.GeneratedPower`))
          (add `/Game/Core/Blueprints/PowerNetwork/PowerNetwork.OnUpdatedDispatcher` _output_get_2 (`|CreateDelegate` :!event `OnNetworkUpdated`)))))))

(event `OnNetworkUpdated`
  (bind _networkref (`self.NetworkRef`))
  (`TextRenderComponent.K2_SetText` (`self.TextRender`) (select `bool` (`self.IsPowered`) :`false` "---" :`true` (`|FormatText` "{Consumed} / {Generated}" (`/Game/Core/Blueprints/PowerNetwork/PowerNetwork.TotalConsumed` _networkref) (`/Game/Core/Blueprints/PowerNetwork/PowerNetwork.TotalGenerated` _networkref)))))

(event `InteractionInterface.BeginInteraction`
  (params (Info :type "InteractionInfo Structure"))
  (set `self.IsPowered` (not (`self.IsPowered`)))
  (bind _network (`self.GetPoweredNetwork`))
  (`/Game/Core/Blueprints/PowerNetwork/PowerNetwork.Recalculate` _network)
  (`self.UpdateGraphics`))

(fn `CanInteract`
  (params (Info :type "InteractionInfo Structure"))
  (returns (ReturnValue :type Boolean))
  (return true))

(fn `GetIsPowerActive`
  (params (InstigatingActor :type "Actor Object Reference"))
  (returns (IsActive :type Boolean))
  (return (`self.IsPowered`)))

(fn `GetIsReceivingPower`
  (returns (IsRecievingPower :type Boolean))
  (return false))

(fn `GetMaxPower`
  (returns (MaxPower :type Integer))
  (return 0))

(fn `GetPower`
  (returns (Power :type Integer))
  (return (`KismetMathLibrary.SelectInt` (`self.GeneratedPower`) 0 (`self.IsPowered`))))

(fn `GetPoweredNetwork`
  (returns (Network :type "/Game/Core/Blueprints/PowerNetwork/PowerNetwork Object Reference"))
  (`/Engine/EditorBlueprintResources/StandardMacros.IsValid` (`self.NetworkRef`)
    (:`Is Valid`
      _)
    (:`Is Not Valid`
      (bind _returnvalue (`|GenericCreateObject` "/Game/Core/Blueprints/PowerNetwork/PowerNetwork.PowerNetwork_C"))
      (bind _output_get (set `self.NetworkRef` _returnvalue))
      (`/Game/Core/Blueprints/PowerNetwork/PowerNetwork.RegisterGenerator` _output_get self (`self.GeneratedPower`))
      (add `/Game/Core/Blueprints/PowerNetwork/PowerNetwork.OnUpdatedDispatcher` _output_get (`|CreateDelegate` :!event `OnNetworkUpdated`))))
  (return (`self.NetworkRef`)))

(fn `UpdateGraphics`
  (`MaterialInstanceDynamic.SetVectorParameterValue` (`self.IndicatorLight_MAT`) "Color" (`KismetMathLibrary.SelectColor` (struct :`G` 1.0 :`A` 1.0) (struct :`R` 1.0 :`A` 1.0) (`self.IsPowered`))))

(fn `UserConstructionScript`)