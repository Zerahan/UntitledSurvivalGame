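; Interactable chair that lets a survival character sit down and stand back up.
; Interaction is always allowed; it casts the interacting pawn to SurvivalCharacter_BP and calls DoSit with itself.
; SitLocation and StandLocation components supply the sit and stand transforms, with the sit point raised and yawed a quarter turn.
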(event `InteractionInterface.BeginInteraction`
  (params (Info :type "InteractionInfo Structure"))
  (bind _assurvival_character_bp (cast `/Game/Core/Blueprints/SurvivalCharacter_BP` (`.PawnRef` (break `InteractionInfo` Info))))
  (`/Game/Core/Blueprints/SurvivalCharacter_BP.DoSit` _assurvival_character_bp self))

(fn `CanInteract`
  (params (Info :type "InteractionInfo Structure"))
  (returns (ReturnValue :type Boolean))
  (return true))

(fn `GetSitPosition`
  (returns (Location :type "Vector Structure") (Rotation :type "Rotator Structure"))
  (bind _sitlocation (`self.SitLocation`))
  (return (+ (`SceneComponent.K2_GetComponentLocation` _sitlocation) (0.0 0.0 96.0)) (`KismetMathLibrary.MakeRotator` (.roll (`SceneComponent.K2_GetComponentRotation` _sitlocation)) (.pitch (`SceneComponent.K2_GetComponentRotation` _sitlocation)) (+ (.yaw (`SceneComponent.K2_GetComponentRotation` _sitlocation)) 90.0))))

(fn `GetStandPosition`
  (returns (Location :type "Vector Structure") (Rotation :type "Rotator Structure"))
  (bind _standlocation (`self.StandLocation`))
  (return (`SceneComponent.K2_GetComponentLocation` _standlocation) (`SceneComponent.K2_GetComponentRotation` _standlocation)))

(fn `UserConstructionScript`)