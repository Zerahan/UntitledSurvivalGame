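; Interactive patch panel that routes power to attached nodes, each active when the plug at its index has a wire connected.
; Players select one of three movable ports, marked by an arrow, then click a free plug to reattach it and trigger power state updates.
; Construction attempts random initial connections and builds spline-mesh wires, whose endpoints follow reattachments.
; Other power getters are stubs, and the active check prints debug text.
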(event `self.OnInteraction`
  (params (Info :type "InteractionInfo Structure"))
  (bind ((`HitComponent` _hitcomponent)) (break `InteractionInfo` Info))
  (`/Engine/EditorBlueprintResources/StandardMacros.IsValid` (`self.HeldPort`)
    (:`Is Valid`
      (if (and (not (`KismetArrayLibrary.Array_Contains` (`self.PortAttachment`) _hitcomponent)) (`KismetArrayLibrary.Array_Contains` (`self.Plugs`) _hitcomponent))
        (`self.Attach Port to Plug` (`self.HeldPort`) _hitcomponent))
      (`self.SetHeldPort` null))
    (:`Is Not Valid`
      (if (`KismetArrayLibrary.Array_Contains` (`|MakeArray` (`self.WirePort1`) (`self.WirePort2`) (`self.WirePort5`) :!type "SceneComponent Object Reference") _hitcomponent)
        (`self.SetHeldPort` _hitcomponent)))))

(event `InteractionInterface.CancelInteraction`
  (params (Info :type "InteractionInfo Structure"))
  (`parent.CancelInteraction` Info)
  (`self.SetHeldPort` null))

(fn `Attach Port to Plug`
  (params (Port :type "SceneComponent Object Reference") (Plug :type "SceneComponent Object Reference"))
  (locals (LocalBeforeTarget :type "SceneComponent Object Reference"))
  (bind _returnvalue (`KismetArrayLibrary.Array_Find` (`self.Ports`) Port))
  (bind _array (`|MakeArray` (`self.WirePort1`) (`self.WirePort2`) (`self.WirePort5`) :!type "SceneComponent Object Reference"))
  (bind _output (`|GetArrayItem` (`self.PortAttachment`) _returnvalue))
  (`/Engine/EditorBlueprintResources/StandardMacros.IsValid` Port
    (:`Is Valid`
      (if (`KismetArrayLibrary.Array_Contains` _array Port)
        (if (not (`KismetArrayLibrary.Array_Contains` (`self.PortAttachment`) Port))
          (set `local.LocalBeforeTarget` _output)
          (`KismetArrayLibrary.Array_Set` (`self.PortAttachment`) _returnvalue Plug true)
          (message `/Game/Core/Blueprints/PowerNetwork/TestPowerNetworkInterface.UpdatePowerState` (`local.LocalBeforeTarget`))
          (message `/Game/Core/Blueprints/PowerNetwork/TestPowerNetworkInterface.UpdatePowerState` _output)
          (`SplineComponent.SetLocationAtSplinePoint` (`|GetArrayItem` (`|MakeArray` (`self.Spline1`) (`self.Spline2`) (`self.Spline5`)) (`KismetArrayLibrary.Array_Find` _array Port)) 1 (`SceneComponent.K2_GetComponentLocation` Plug) "World" true)
          (`self.UpdateSplines`))))))

(fn `GetIsPowerActive`
  (params (InstigatingActor :type "Actor Object Reference"))
  (returns (IsActive :type Boolean))
  (bind _returnvalue (`KismetArrayLibrary.Array_Find` (`self.AttachedPoweredNodes`) InstigatingActor))
  (bind _output (`|GetArrayItem` (`self.Plugs`) _returnvalue))
  (bind _returnvalue_2 (`KismetArrayLibrary.Array_Contains` (`self.PortAttachment`) _output))
  (`KismetSystemLibrary.PrintText` (`|FormatText` "Attachment at {Index} is {Open} \"{Name}\"" _returnvalue _returnvalue_2 (`KismetSystemLibrary.GetDisplayName` _output)))
  (return _returnvalue_2))

(fn `GetIsReceivingPower`
  (returns (IsRecievingPower :type Boolean))
  (return false))

(fn `GetMaxPower`
  (returns (MaxPower :type Integer))
  (return 0))

(fn `GetPower`
  (returns (Power :type Integer))
  (return 0))

(fn `GetPoweredNetwork`
  (returns (Network :type "/Game/Core/Blueprints/PowerNetwork/PowerNetwork Object Reference"))
  (return null))

(fn `SetHeldPort`
  (params (HeldPort :type "SceneComponent Object Reference"))
  (bind _output_get (set `self.HeldPort` HeldPort))
  (`SceneComponent.SetHiddenInGame` (`self.ArrowPort`) (not (`KismetSystemLibrary.IsValid` _output_get)) false)
  (`/Engine/EditorBlueprintResources/StandardMacros.IsValid` _output_get
    (:`Is Valid`
      (`SceneComponent.K2_SetRelativeLocation` (`self.ArrowPort`) (+ (`SceneComponent.RelativeLocation` HeldPort) (0.0 -20.0 0.0)) false false))))

(fn `UpdateSplines`
  (for _array_element (`|MakeArray` (`self.Spline1`) (`self.Spline2`) (`self.Spline5`))
    (for _index (range (+ (- (`SplineComponent.GetNumberOfSplinePoints` _array_element) 2) 1))
      (bind _asspline_mesh_component (cast `SplineMeshComponent` (`SceneComponent.GetChildComponent` _array_element _index)))
      (bind (_location _tangent) (`SplineComponent.GetLocationAndTangentAtSplinePoint` _array_element _index "Local"))
      (bind (_location_2 _tangent_2) (`SplineComponent.GetLocationAndTangentAtSplinePoint` _array_element (+ _index 1) "Local"))
      (`SplineMeshComponent.SetStartAndEnd` _asspline_mesh_component _location _tangent _location_2 _tangent_2 true))))

(fn `UserConstructionScript`
  (locals (NewLocalVar :type "SplineComponent Object Reference"))
  (`|ExecutionSequence`
    (:`then_0`
      (set `self.Plugs` (`|MakeArray` (`self.WirePlug1`) (`self.WirePlug2`) (`self.WirePlug3`) (`self.WirePlug4`) (`self.WirePlug5`) (`self.WirePlug6`) :!type "SceneComponent Object Reference"))
      (set `self.Ports` (`|MakeArray` (`self.WirePort1`) (`self.WirePort2`) (`self.WirePort3`) (`self.WirePort4`) (`self.WirePort5`) (`self.WirePort6`) :!type "SceneComponent Object Reference"))
      (`self.Attach Port to Plug` (`self.WirePort1`) (`KismetArrayLibrary.Array_Random` (`self.Plugs`)))
      (`self.Attach Port to Plug` (`self.WirePort2`) (`KismetArrayLibrary.Array_Random` (`self.Plugs`)))
      (`self.Attach Port to Plug` (`self.WirePort5`) (`KismetArrayLibrary.Array_Random` (`self.Plugs`))))
    (:`then_1`
      (for _array_element (`|MakeArray` (`self.Spline1`) (`self.Spline2`) (`self.Spline5`))
        (for _index (range (+ (- (`SplineComponent.GetNumberOfSplinePoints` _array_element) 2) 1))
          (bind _returnvalue (`AddComponent|NODE_AddSplineMeshComponent-0` :`RelativeTransform` (`KismetMathLibrary.MakeTransform` (0.0 0.0 0.0))))
          (bind (_location _tangent) (`SplineComponent.GetLocationAndTangentAtSplinePoint` _array_element _index "Local"))
          (bind (_location_2 _tangent_2) (`SplineComponent.GetLocationAndTangentAtSplinePoint` _array_element (+ _index 1) "Local"))
          (`SplineMeshComponent.SetStartAndEnd` _returnvalue _location _tangent _location_2 _tangent_2 true)
          (`SceneComponent.K2_AttachToComponent` _returnvalue _array_element "None" "KeepRelative" "KeepRelative" "KeepRelative" true))))))