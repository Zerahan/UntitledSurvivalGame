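; Development map generator Blueprint that extends a parent generator for building maps from rooms with doors.
; BeginPlay fills MeshesToUse with meshes, doors and sizes from a DataTable before calling the parent.
; GenerateNextRoom prints a running room count and defers to the parent, leaving its older Blueprint door-matching logic disconnected.
; MakeRoom builds a room tile with two fixed opposite doors and up to four random extra doors, positioned by TileSize.
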(event `self.ReceiveBeginPlay`
  (bind _outrownames (`DataTableFunctionLibrary.GetDataTableRowNames` (`self.Data Table`)))
  (for _array_element _outrownames
    (bind _returnvalue (`|GetDataTableRow` (`self.Data Table`) _array_element)
      (:`then`
        (bind (_mesh _doors _sizes) (break `/Game/Dev/MeshDataStruct_BP` _returnvalue))
        (`KismetArrayLibrary.Array_Add` (`self.MeshesToUse`) (make `MeshData` _mesh _doors _sizes)))))
  (`parent.ReceiveBeginPlay`))

(fn `GenerateNextRoom`
  (returns (ReturnValue :type Boolean))
  (locals (NextDoor :type "DoorTile Structure") (DoorIndex :type Integer) (Doors :type "Array of DoorTile Structure") (Room :type "RoomTile Structure") (TrimmedList :type "Array of Integer"))
  (`/Engine/EditorBlueprintResources/StandardMacros.IncrementInt` (`self.RoomCounter`)
    (:`  `
      (`KismetSystemLibrary.PrintText` (`|FormatText` "Generated Room # {Number}" (`self.RoomCounter`)))
      (bind _returnvalue (`parent.GenerateNextRoom`))
      (return _returnvalue))))

(fn `MakeRoom`
  (returns (RoomTile :type "RoomTile Structure"))
  (locals (Doors :type "Array of DoorTile Structure"))
  (bind _returnvalue (`KismetMathLibrary.Conv_IntToDouble` (`self.TileSize`)))
  (bind _returnvalue_2 (`KismetMathLibrary.Conv_IntToDouble` (`self.TileSize`)))
  (bind _returnvalue_3 (`KismetMathLibrary.Conv_IntToDouble` (`self.TileSize`)))
  (bind _returnvalue_4 (`KismetMathLibrary.Conv_IntToDouble` (`self.TileSize`)))
  (`|ExecutionSequence`
    (:`then_0`
      (set `local.Doors` (`|MakeArray` (make `DoorTile` (`KismetMathLibrary.MakeVector` 0.0 (* (`KismetMathLibrary.Conv_IntToDouble` (`self.TileSize`)) 2.0)) (`KismetMathLibrary.Conv_VectorToRotator` (`KismetMathLibrary.GetRightVector` (struct)))) (make `DoorTile` (`KismetMathLibrary.MakeVector` 0.0 (* (`KismetMathLibrary.Conv_IntToDouble` (`self.TileSize`)) -2.0)) (`KismetMathLibrary.Conv_VectorToRotator` (* (`KismetMathLibrary.GetRightVector` (struct)) -1.0)) 1)))
      (`|ExecutionSequence`
        (:`then_0`
          (if (`KismetMathLibrary.RandomBool`)
            (`KismetArrayLibrary.Array_Add` (`local.Doors`) (make `DoorTile` (`KismetMathLibrary.MakeVector` (* _returnvalue_2 -1.0) _returnvalue_2) (`KismetMathLibrary.Conv_VectorToRotator` (* (`KismetMathLibrary.GetForwardVector` (struct)) -1.0)) (`KismetMathLibrary.Conv_IntToByte` (`KismetMathLibrary.RandomIntegerInRange` 0 1))))))
        (:`then_1`
          (if (`KismetMathLibrary.RandomBool`)
            (`KismetArrayLibrary.Array_Add` (`local.Doors`) (make `DoorTile` (`KismetMathLibrary.MakeVector` (* _returnvalue_3 -1.0) (* _returnvalue_3 -1.0)) (`KismetMathLibrary.Conv_VectorToRotator` (* (`KismetMathLibrary.GetForwardVector` (struct)) -1.0)) (`KismetMathLibrary.Conv_IntToByte` (`KismetMathLibrary.RandomIntegerInRange` 0 1))))))
        (:`then_2`
          (if (`KismetMathLibrary.RandomBool`)
            (`KismetArrayLibrary.Array_Add` (`local.Doors`) (make `DoorTile` (`KismetMathLibrary.MakeVector` _returnvalue_4 _returnvalue_4) (`KismetMathLibrary.Conv_VectorToRotator` (* (`KismetMathLibrary.GetForwardVector` (struct)) -1.0)) (`KismetMathLibrary.Conv_IntToByte` (`KismetMathLibrary.RandomIntegerInRange` 0 1))))))
        (:`then_3`
          (if (`KismetMathLibrary.RandomBool`)
            (`KismetArrayLibrary.Array_Add` (`local.Doors`) (make `DoorTile` (`KismetMathLibrary.MakeVector` _returnvalue (* _returnvalue -1.0)) (`KismetMathLibrary.Conv_VectorToRotator` (* (`KismetMathLibrary.GetForwardVector` (struct)) -1.0)) (`KismetMathLibrary.Conv_IntToByte` (`KismetMathLibrary.RandomIntegerInRange` 0 1))))))))
    (:`then_1`
      (return (make `RoomTile` :`Doors` (`local.Doors`))))))

(fn `UserConstructionScript`)