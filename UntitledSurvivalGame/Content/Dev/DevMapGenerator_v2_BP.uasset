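; Development map generator Blueprint that drives tile-based room generation and reports progress through debug text.
; BeginPlay fills the tile shape and mesh arrays from a shapes data table.
; Tick makes a single GenerateTileIterator attempt, updates and prints the generated room count, then calls the parent Tick.
; Tile cleanup, path fixing and a direction-vector rotation debug print are present but disconnected.
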(event `self.ReceiveTick`
  (params (DeltaSeconds :type "Float (single-precision)"))
  (bind _generatedroomcount (`self.GeneratedRoomCount`))
  (`|ExecutionSequence`
    (:`then_0`
      (if (< (`self.AttemptCount`) 1)
        (`/Engine/EditorBlueprintResources/StandardMacros.IncrementInt` (`self.AttemptCount`)
          (:`  `
            (bind _returnvalue (`self.GenerateTileIterator`))
            (if _returnvalue
              (`/Engine/EditorBlueprintResources/StandardMacros.IncrementInt` _generatedroomcount
                (:`  `
                  _)))
            (`KismetSystemLibrary.PrintText` (`|FormatText` "Generated room: {Num}" _generatedroomcount))))))
    (:`then_1`
      (`parent.ReceiveTick` DeltaSeconds))))

(event `self.ReceiveBeginPlay`
  (`|ExecutionSequence`
    (:`then_0`
      (`KismetArrayLibrary.Array_Clear` (`self.TileShapes`))
      (bind _outrownames (`DataTableFunctionLibrary.GetDataTableRowNames` (`self.ShapesTable`)))
      (for _array_element _outrownames
        (bind _returnvalue (`|GetDataTableRow` (`self.ShapesTable`) _array_element)
          (:`then`
            (bind (_mesh _shape) (break `/Game/Dev/ShapeData_BP` _returnvalue))
            (`KismetArrayLibrary.Array_Add` (`self.TileShapes`) _shape)
            (`KismetArrayLibrary.Array_Add` (`self.Mesh`) _mesh)))))))

(fn `UserConstructionScript`)